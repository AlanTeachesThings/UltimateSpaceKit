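; Test Blueprint for a modular environment grid that previews a room's floor as tiles coloured by whether they are blocked.
; The construction script derives the room size from SizeControl and GridSize, then spawns grid-snapped floor meshes centred on the actor, each with its own dynamic material.
; Tiles and their materials are stored in maps, then each tile runs a slightly shrunken box overlap test, turning red on overlap and green otherwise.
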(fn `ActualRoomSize`
  (returns (ActualRoomSize :type "Vector2D Structure"))
  (bind (_gridsize_x _gridsize_y) (`KismetMathLibrary.BreakVector` (`self.GridSize`)))
  (return (* (`self.RoomSize`) (`KismetMathLibrary.MakeVector2D` _gridsize_x _gridsize_y))))

(fn `CheckTileCollision`
  (params (TileToCheck :type "StaticMeshComponent Object Reference"))
  (returns (Overlap :type Boolean))
  (locals (OverlapFound :type Boolean))
  (bind (_origin _boxextent) (`KismetSystemLibrary.GetComponentBounds` TileToCheck))
  (bind _outcomponents (`KismetSystemLibrary.BoxOverlapComponents` _origin (* _boxextent 0.9) (`|MakeArray` "ObjectTypeQuery1" "ObjectTypeQuery2" :!type "EObjectTypeQuery Enum")))
  (set `local.OverlapFound` false)
  (for _array_element _outcomponents
    (if (not (== TileToCheck _array_element))
      (set `local.OverlapFound` true)))
  (return (`local.OverlapFound`)))

(fn `FitLocationToGrid`
  (params (LocationIn :type "Vector Structure"))
  (returns (LocationOut :type "Vector Structure"))
  (bind _gridsize (`self.GridSize`))
  (bind (_returnvalue_x _returnvalue_y _returnvalue_z) (`KismetMathLibrary.BreakVector` (/ LocationIn _gridsize)))
  (return (* (`KismetMathLibrary.MakeVector` (`KismetMathLibrary.Conv_IntToDouble` (`KismetMathLibrary.Round` _returnvalue_x)) (`KismetMathLibrary.Conv_IntToDouble` (`KismetMathLibrary.Round` _returnvalue_y)) (`KismetMathLibrary.Conv_IntToDouble` (`KismetMathLibrary.Round` _returnvalue_z))) _gridsize)))

(fn `GridLocation`
  (returns (GridLocation :type "Vector Structure"))
  (return (`self.FitLocationToGrid` (`self.K2_GetActorLocation`))))

(fn `GridOffset`
  (returns (GridOffset :type "Vector2D Structure"))
  (return (/ (`self.ActualRoomSize`) (2.0 2.0))))

(fn `RoomSize`
  (returns (RoomSize :type "Vector2D Structure"))
  (bind (_roomsize_x _roomsize_y) (`KismetMathLibrary.BreakVector` (`self.RoomSize3D`)))
  (return (`KismetMathLibrary.MakeVector2D` _roomsize_x _roomsize_y)))

(fn `RoomSize3D`
  (returns (RoomSize :type "Vector Structure"))
  (bind (_returnvalue_x _returnvalue_y _returnvalue_z) (`KismetMathLibrary.BreakVector` (/ (* (`self.SizeControl`) (2.0 2.0 1.0)) (`self.GridSize`))))
  (return (`KismetMathLibrary.MakeVector` (`KismetMathLibrary.Conv_IntToDouble` (`KismetMathLibrary.Round` _returnvalue_x)) (`KismetMathLibrary.Conv_IntToDouble` (`KismetMathLibrary.Round` _returnvalue_y)) (`KismetMathLibrary.Conv_IntToDouble` (`KismetMathLibrary.Round` _returnvalue_z)))))

(fn `UpdateAllTileColours`
  (bind _values (`BlueprintMapLibrary.Map_Values` (`self.Tiles`)))
  (for _array_element _values
    (`self.UpdateTileColour` _array_element)))

(fn `UpdateTileColour`
  (params (InputPin :type "StaticMeshComponent Object Reference"))
  (bind _value (`BlueprintMapLibrary.Map_Find` (`self.Materials`) InputPin))
  (bind _overlap (`self.CheckTileCollision` InputPin))
  (if _overlap
    (`MaterialInstanceDynamic.SetVectorParameterValue` _value "Colour" (struct :`R` 1.0 :`A` 1.0))
    (`KismetSystemLibrary.PrintString` "Hello")
    (else
      (`MaterialInstanceDynamic.SetVectorParameterValue` _value "Colour" (struct :`G` 1.0 :`A` 1.0)))))

(fn `UserConstructionScript`
  (bind (_gridoffset_x _gridoffset_y) (`KismetMathLibrary.BreakVector2D` (`self.GridOffset`)))
  (bind (_roomsize_x _roomsize_y) (`KismetMathLibrary.BreakVector2D` (`self.RoomSize`)))
  (bind _roomsize_x_2 (`KismetMathLibrary.BreakVector2D` (`self.RoomSize`)))
  (bind _gridsize_x (`KismetMathLibrary.BreakVector` (`self.GridSize`)))
  (bind (_gridsize_x_2 _gridsize_y) (`KismetMathLibrary.BreakVector` (`self.GridSize`)))
  (`|ExecutionSequence`
    (:`then_0`
      (for _index (range (+ (`KismetMathLibrary.FTrunc` (- _roomsize_x_2 1.0)) 1))
        (for _index_2 (range (+ (`KismetMathLibrary.FTrunc` (- _roomsize_y 1.0)) 1))
          (bind _returnvalue (`AddComponent|NODE_AddStaticMeshComponent-0`))
          (`StaticMeshComponent.SetStaticMesh` _returnvalue "/Game/ModularEnv/Meshes/GridFloorBasic.GridFloorBasic")
          (`SceneComponent.K2_SetWorldLocation` _returnvalue (`self.FitLocationToGrid` (+ (`self.K2_GetActorLocation`) (`KismetMathLibrary.MakeVector` (- (* _index _gridsize_x) _gridoffset_x) (- (* _index_2 _gridsize_y) _gridoffset_y)))) false false)
          (bind _returnvalue_2 (`KismetMaterialLibrary.CreateDynamicMaterialInstance` "/Game/ModularEnv/RoomGenOld/RoomPreview_M.RoomPreview_M"))
          (`BlueprintMapLibrary.Map_Add` (`self.Materials`) _returnvalue _returnvalue_2)
          (`PrimitiveComponent.SetMaterial` _returnvalue 0 _returnvalue_2)
          (`BlueprintMapLibrary.Map_Add` (`self.Tiles`) (`KismetMathLibrary.MakeVector2D` (`KismetMathLibrary.Conv_IntToDouble` _index) (`KismetMathLibrary.Conv_IntToDouble` _index_2)) _returnvalue))))
    (:`then_1`
      (`self.UpdateAllTileColours`))))