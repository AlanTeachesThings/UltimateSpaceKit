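; Modular room actor that assembles a floor, walls and corner columns from RoomSize and TileSize in the construction script.
; It lays a grid of floor meshes around the actor, storing them by grid coordinate so edge and corner passes can swap and rotate them.
; Wall and column helpers run per side or corner using North/East flags.
; Edge loops use only RoomSize.Y and wall counts only RoomSize.X, effectively assuming square rooms.
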(fn `AddFloorTile`
  (params (FloorTileClass :type "StaticMesh Object Reference"))
  (returns (FloorTileActor :type "Actor Object Reference"))
  (bind _returnvalue (`|SpawnActorFromClass` "/Script/Engine.StaticMeshActor" (`KismetMathLibrary.MakeTransform` (0.0 0.0 0.0)) "Undefined" "OverrideRootScale" null null))
  (`StaticMeshComponent.SetStaticMesh` (`StaticMeshActor.StaticMeshComponent` _returnvalue) FloorTileClass)
  (return _returnvalue))

(fn `Columns`
  (params (North :type Boolean) (East :type Boolean))
  (bind (_tilesize_x _tilesize_y) (`KismetMathLibrary.BreakVector2D` (`self.TileSize`)))
  (bind (_returnvalue_x _returnvalue_y) (`KismetMathLibrary.BreakVector2D` (- (+ (`self.GridOffset`) (`KismetMathLibrary.MakeVector2D` (`KismetMathLibrary.SelectFloat` 0.0 _tilesize_x North) (`KismetMathLibrary.SelectFloat` 0.0 _tilesize_y East))) (/ (`self.TileSize`) (2.0 2.0)))))
  (bind (_returnvalue_x_2 _returnvalue_y_2) (`KismetMathLibrary.BreakVector2D` (`KismetMathLibrary.MakeVector2D` _returnvalue_x _returnvalue_y)))
  (bind _returnvalue (`AddComponent|NODE_AddStaticMeshComponent-3` :`RelativeTransform` (`KismetMathLibrary.MakeTransform` (+ (`KismetMathLibrary.MakeVector` (`KismetMathLibrary.SelectFloat` _returnvalue_x_2 (* _returnvalue_x_2 -1.0) North) (`KismetMathLibrary.SelectFloat` _returnvalue_y_2 (* _returnvalue_y_2 -1.0) East)) (`KismetMathLibrary.MakeVector` (`KismetMathLibrary.SelectFloat` -25.0 25.0 North) (`KismetMathLibrary.SelectFloat` -25.0 25.0 East))))))
  (`StaticMeshComponent.SetStaticMesh` _returnvalue "/Game/ModularEnv/Meshes/Column_1.Column_1"))

(fn `FloorCorners`
  (params (North :type Boolean) (East :type Boolean))
  (bind (_roomsize_x _roomsize_y) (`KismetMathLibrary.BreakVector2D` (`self.RoomSize`)))
  (bind _value (`BlueprintMapLibrary.Map_Find` (`self.FloorTiles`) (`KismetMathLibrary.MakeVector2D` (`KismetMathLibrary.SelectFloat` (- _roomsize_x 1.0) 0.0 North) (`KismetMathLibrary.SelectFloat` (- _roomsize_y 1.0) 0.0 East))))
  (`StaticMeshComponent.SetStaticMesh` _value "/Game/ModularEnv/Meshes/FloorTile_Corner_FloorTile_Corner.FloorTile_Corner_FloorTile_Corner")
  (`SceneComponent.K2_SetRelativeRotation` _value (`KismetMathLibrary.MakeRotator` 0.0 0.0 (`KismetMathLibrary.SelectFloat` (`KismetMathLibrary.SelectFloat` -90.0 0.0 North) (`KismetMathLibrary.SelectFloat` 180.0 90.0 North) East)) false false))

(fn `FloorEdges`
  (params (North :type Boolean) (East :type Boolean))
  (bind (_roomsize_x _roomsize_y) (`KismetMathLibrary.BreakVector2D` (`self.RoomSize`)))
  (bind _returnvalue (- _roomsize_y 1.0))
  (bind _returnvalue_2 (`KismetMathLibrary.SelectFloat` 0.0 _returnvalue North))
  (for _index (range (+ (`KismetMathLibrary.FTrunc` _returnvalue) 1))
    (bind _returnvalue_3 (`KismetMathLibrary.Conv_IntToDouble` _index))
    (bind _value (`BlueprintMapLibrary.Map_Find` (`self.FloorTiles`) (`KismetMathLibrary.MakeVector2D` (`KismetMathLibrary.SelectFloat` _returnvalue_2 _returnvalue_3 East) (`KismetMathLibrary.SelectFloat` _returnvalue_3 _returnvalue_2 East))))
    (`SceneComponent.K2_SetRelativeRotation` _value (`KismetMathLibrary.MakeRotator` 0.0 0.0 (`KismetMathLibrary.SelectFloat` (`KismetMathLibrary.SelectFloat` 90.0 -90.0 North) (`KismetMathLibrary.SelectFloat` 180.0 0.0 North) East)) false false)
    (`StaticMeshComponent.SetStaticMesh` _value "/Game/ModularEnv/Meshes/FloorTile_Side_FloorTile_Side.FloorTile_Side_FloorTile_Side")))

(fn `GridOffset`
  (returns (ReturnValue :type "Vector2D Structure"))
  (return (/ (`self.GridSize`) (2.0 2.0))))

(fn `GridSize`
  (returns (ReturnValue :type "Vector2D Structure"))
  (return (* (`self.RoomSize`) (`self.TileSize`))))

(fn `SetUpRoom`)

(fn `UserConstructionScript`
  (bind (_returnvalue_x _returnvalue_y) (`KismetMathLibrary.BreakVector2D` (`self.GridOffset`)))
  (bind (_tilesize_x _tilesize_y) (`KismetMathLibrary.BreakVector2D` (`self.TileSize`)))
  (bind (_roomsize_x _roomsize_y) (`KismetMathLibrary.BreakVector2D` (`self.RoomSize`)))
  (`|ExecutionSequence`
    (:`then_0`
      ;[1 1 1] Floor (Basic Tiles Only)
      (for _index (range (+ (`KismetMathLibrary.FTrunc` (- _roomsize_y 1.0)) 1))
        (for _index_2 (range (+ (`KismetMathLibrary.FTrunc` (- _roomsize_x 1.0)) 1))
          (bind _returnvalue (`AddComponent|NODE_AddStaticMeshComponent-1`))
          (`StaticMeshComponent.SetStaticMesh` _returnvalue "/Game/ModularEnv/Meshes/FloorTile_Basic_FloorTile_Basic.FloorTile_Basic_FloorTile_Basic")
          (`SceneComponent.K2_SetWorldLocation` _returnvalue (+ (`self.K2_GetActorLocation`) (`KismetMathLibrary.MakeVector` (- (* _index_2 _tilesize_x) _returnvalue_x) (- (* _index _tilesize_y) _returnvalue_y))) false false)
          (`BlueprintMapLibrary.Map_Add` (`self.FloorTiles`) (`KismetMathLibrary.MakeVector2D` (`KismetMathLibrary.Conv_IntToDouble` _index_2) (`KismetMathLibrary.Conv_IntToDouble` _index)) _returnvalue))))
    (:`then_1`
      ;[1 1 1] Floor Edges
      (`self.FloorEdges` false)
      (`self.FloorEdges` true)
      (`self.FloorEdges` false true)
      (`self.FloorEdges` true true))
    (:`then_2`
      ;[1 1 1] Floor Corners
      (`self.FloorCorners` false)
      (`self.FloorCorners` true)
      (`self.FloorCorners` false true)
      (`self.FloorCorners` true true))
    (:`then_3`
      ;[1 1 1] Walls
      (`self.WallSetup` false true)
      (`self.WallSetup` true true)
      (`self.WallSetup` true)
      (`self.WallSetup` false))
    (:`then_4`
      ;[1 1 1] Columns
      (`self.Columns` false)
      (`self.Columns` true)
      (`self.Columns` false true)
      (`self.Columns` true true))))

(fn `WallSetup`
  (params (North :type Boolean) (East :type Boolean))
  (locals (NorthLocal :type Boolean) (EastLocal :type Boolean))
  (bind (_roomsize_x _roomsize_y) (`KismetMathLibrary.BreakVector2D` (`self.RoomSize`)))
  (bind _roomsize_x_2 (`KismetMathLibrary.BreakVector2D` (`self.RoomSize`)))
  (bind _tilesize_x (`KismetMathLibrary.BreakVector2D` (`self.TileSize`)))
  (bind (_roomsize_x_3 _roomsize_y_2) (`KismetMathLibrary.BreakVector2D` (`self.RoomSize`)))
  (bind _northlocal (`local.NorthLocal`))
  (bind (_roomsize_x_4 _roomsize_y_3) (`KismetMathLibrary.BreakVector2D` (`self.RoomSize`)))
  (bind _wallsize (`self.WallSize`))
  (bind _tilesize_x_2 (`KismetMathLibrary.BreakVector2D` (`self.TileSize`)))
  (bind _returnvalue (/ _tilesize_x_2 (`self.WallSize`)))
  (bind _returnvalue_2 (* (* _wallsize (/ (* (- _roomsize_y (`KismetMathLibrary.SelectFloat` 1.0 -1.0 (`local.NorthLocal`))) _returnvalue) 2.0)) (`KismetMathLibrary.SelectFloat` 1.0 -1.0 (`local.NorthLocal`))))
  (set `local.EastLocal` East)
  (set `local.NorthLocal` North)
  (for _index (range (+ (`KismetMathLibrary.FTrunc` (- (* _roomsize_x_2 (/ _tilesize_x (`self.WallSize`))) 1.0)) 1))
    (bind _returnvalue_3 (`AddComponent|NODE_AddStaticMeshComponent-2`))
    (`StaticMeshComponent.SetStaticMesh` _returnvalue_3 "/Game/ModularEnv/Walls/Wall_1.Wall_1")
    (bind _returnvalue_4 (- (* _index _wallsize) (* _wallsize (/ (* (- _roomsize_x (`KismetMathLibrary.SelectFloat` 1.0 1.0 (`local.EastLocal`))) _returnvalue) 2.0))))
    (`SceneComponent.K2_SetWorldLocationAndRotation` _returnvalue_3 (+ (`self.K2_GetActorLocation`) (`KismetMathLibrary.MakeVector` (`KismetMathLibrary.SelectFloat` _returnvalue_4 _returnvalue_2 (`local.EastLocal`)) (`KismetMathLibrary.SelectFloat` _returnvalue_2 _returnvalue_4 (`local.EastLocal`)))) (`KismetMathLibrary.MakeRotator` 0.0 0.0 (`KismetMathLibrary.SelectFloat` (`KismetMathLibrary.SelectFloat` -90.0 90.0 _northlocal) (`KismetMathLibrary.SelectFloat` 180.0 0.0 _northlocal) (`local.EastLocal`))) false false)
    (`BlueprintMapLibrary.Map_Add` (`self.Walls`) (`KismetMathLibrary.MakeVector2D` (`KismetMathLibrary.SelectFloat` (`KismetMathLibrary.Conv_IntToDouble` _index) (`KismetMathLibrary.SelectFloat` 0.0 (- _roomsize_y_3 1.0) (`local.EastLocal`)) (`local.NorthLocal`)) (`KismetMathLibrary.SelectFloat` (`KismetMathLibrary.Conv_IntToDouble` _index) (`KismetMathLibrary.SelectFloat` 0.0 (- _roomsize_y_2 1.0) (`local.NorthLocal`)) (`local.EastLocal`))) _returnvalue_3)))