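; Room generator Blueprint that assembles a modular preview room, centred on the actor, from a RoomSize grid in its construction script.
; It adds floor tiles, walls and corner columns as static mesh components using RoomPreview_M.
; Edge and corner passes look up FloorTiles0 to swap and rotate meshes, but the node filling that map is disconnected.
; BeginPlay creates green/red preview materials for an overlap check that is also disconnected.
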(event `self.ReceiveBeginPlay`
  (bind _returnvalue (`KismetMaterialLibrary.CreateDynamicMaterialInstance` "/Game/ModularEnv/RoomPreview_M.RoomPreview_M"))
  (set `self.GreenMat` _returnvalue)
  (bind _returnvalue_2 (`KismetMaterialLibrary.CreateDynamicMaterialInstance` "/Game/ModularEnv/RoomPreview_M.RoomPreview_M"))
  (bind _output_get (set `self.RedMat` _returnvalue_2))
  (`MaterialInstanceDynamic.SetVectorParameterValue` _output_get "Colour" (struct :`R` 1.0 :`A` 1.0)))

(event `self.ReceiveTick`
  (params (DeltaSeconds :type "Float (single-precision)")))

(fn `ActualFloorSize`
  (returns (FloorSize :type "Vector2D Structure"))
  (return (* (* (`self.RoomSize`) (2.0 2.0)) (`self.TileSize`))))

(fn `Colums`
  (params (Right :type Boolean) (Upper :type Boolean))
  (bind (_floorsize_x _floorsize_y) (`KismetMathLibrary.BreakVector2D` (`self.ActualFloorSize`)))
  (bind (_offset_x _offset_y) (`KismetMathLibrary.BreakVector2D` (`self.GridOffset`)))
  (bind (_tilesize_x _tilesize_y) (`KismetMathLibrary.BreakVector2D` (`self.TileSize`)))
  (bind _returnvalue (`AddComponent|NODE_AddStaticMeshComponent-8` :`RelativeTransform` (`KismetMathLibrary.MakeTransform` (`KismetMathLibrary.MakeVector` (- (- (`KismetMathLibrary.SelectFloat` (+ _floorsize_x -25.0) 25.0 Right) _offset_x) (/ _tilesize_x 2.0)) (- (- (`KismetMathLibrary.SelectFloat` (- _floorsize_y 25.0) 25.0 Upper) _offset_y) (/ _tilesize_y 2.0))))))
  (`StaticMeshComponent.SetStaticMesh` _returnvalue "/Game/ModularEnv/Meshes/Column_1.Column_1")
  (`PrimitiveComponent.SetMaterial` _returnvalue 0 "/Game/ModularEnv/RoomPreview_M.RoomPreview_M"))

(fn `FloorCorners`
  (params (Upper :type Boolean) (Right :type Boolean))
  (bind (_returnvalue_x _returnvalue_y) (`KismetMathLibrary.BreakVector2D` (* (`self.RoomSize`) (2.0 2.0))))
  (bind _value (`BlueprintMapLibrary.Map_Find` (`self.FloorTiles_0`) (`KismetMathLibrary.MakeVector2D` (`KismetMathLibrary.SelectFloat` 0.0 (- _returnvalue_x 1.0) Right) (`KismetMathLibrary.SelectFloat` (- _returnvalue_y 1.0) 0.0 Upper))))
  (`StaticMeshComponent.SetStaticMesh` _value "/Game/ModularEnv/Meshes/FloorTile_Corner_FloorTile_Corner.FloorTile_Corner_FloorTile_Corner")
  (`SceneComponent.K2_SetRelativeRotation` _value (`KismetMathLibrary.MakeRotator` 0.0 0.0 (`KismetMathLibrary.SelectFloat` (`KismetMathLibrary.SelectFloat` 0.0 -90.0 Right) (`KismetMathLibrary.SelectFloat` 90.0 180.0 Right) Upper)) false false))

(fn `FloorEdges`
  (params (Horixzontal :type Boolean) (UpOrRight :type Boolean))
  (locals (Horizontal_Local :type Boolean) (UpRightLocal :type Boolean))
  (bind _horizontal_local (`local.Horizontal_Local`))
  (bind _uprightlocal (`local.UpRightLocal`))
  (bind (_returnvalue_x _returnvalue_y) (`KismetMathLibrary.BreakVector2D` (* (`self.RoomSize`) (2.0 2.0))))
  (set `local.Horizontal_Local` Horixzontal)
  (set `local.UpRightLocal` UpOrRight)
  (for _index (range (+ (`KismetMathLibrary.FTrunc` (- (`KismetMathLibrary.SelectFloat` _returnvalue_x _returnvalue_y (`local.Horizontal_Local`)) 1.0)) 1))
    (bind _returnvalue (`KismetMathLibrary.Conv_IntToDouble` _index))
    (bind _value (`BlueprintMapLibrary.Map_Find` (`self.FloorTiles_0`) (`KismetMathLibrary.MakeVector2D` (`KismetMathLibrary.SelectFloat` _returnvalue (`KismetMathLibrary.SelectFloat` 0.0 (- _returnvalue_x 1.0) (`local.UpRightLocal`)) _horizontal_local) (`KismetMathLibrary.SelectFloat` (`KismetMathLibrary.SelectFloat` 0.0 (- _returnvalue_y 1.0) (`local.UpRightLocal`)) _returnvalue _horizontal_local))))
    (`SceneComponent.K2_SetRelativeRotation` _value (`KismetMathLibrary.MakeRotator` 0.0 0.0 (`KismetMathLibrary.SelectFloat` (`KismetMathLibrary.SelectFloat` 180.0 0.0 _uprightlocal) (`KismetMathLibrary.SelectFloat` 90.0 -90.0 _uprightlocal) (`local.Horizontal_Local`))) false false)
    (`StaticMeshComponent.SetStaticMesh` _value "/Game/ModularEnv/Meshes/FloorTile_Side_FloorTile_Side.FloorTile_Side_FloorTile_Side")))

(fn `GridOffset`
  (returns (Offset :type "Vector2D Structure"))
  (return (/ (- (`self.ActualFloorSize`) (`self.TileSize`)) (2.0 2.0))))

(fn `UserConstructionScript`
  (bind (_offset_x _offset_y) (`KismetMathLibrary.BreakVector2D` (`self.GridOffset`)))
  (bind (_tilesize_x _tilesize_y) (`KismetMathLibrary.BreakVector2D` (`self.TileSize`)))
  (bind (_returnvalue_x _returnvalue_y) (`KismetMathLibrary.BreakVector2D` (* (`self.RoomSize`) (2.0 2.0))))
  (`|ExecutionSequence`
    (:`then_0`
      ;[1 1 1] Floor Tiles
      (for _index (range (+ (`KismetMathLibrary.FTrunc` (- _returnvalue_y 1.0)) 1))
        (for _index_2 (range (+ (`KismetMathLibrary.FTrunc` (- _returnvalue_x 1.0)) 1))
          (bind _returnvalue (`AddComponent|NODE_AddStaticMeshComponent-9` :`RelativeTransform` (`KismetMathLibrary.MakeTransform` (`KismetMathLibrary.MakeVector` (- (* _index_2 _tilesize_x) _offset_x) (- (* _index _tilesize_y) _offset_y)))))
          (`StaticMeshComponent.SetStaticMesh` _returnvalue "/Game/ModularEnv/Meshes/FloorTile_Basic_FloorTile_Basic.FloorTile_Basic_FloorTile_Basic")
          (`PrimitiveComponent.SetMaterial` _returnvalue 0 "/Game/ModularEnv/RoomPreview_M.RoomPreview_M")
          (`PrimitiveComponent.SetCollisionResponseToAllChannels` _returnvalue "ECR_Overlap"))))
    (:`then_1`
      (`self.FloorEdges` false)
      (`self.FloorEdges` true)
      (`self.FloorEdges` false true)
      (`self.FloorEdges` true true))
    (:`then_2`
      (`self.FloorCorners` false)
      (`self.FloorCorners` true)
      (`self.FloorCorners` false true)
      (`self.FloorCorners` true true))
    (:`then_3`
      (`self.WallSetup` false)
      (`self.WallSetup` true)
      (`self.WallSetup` false true)
      (`self.WallSetup` true true))
    (:`then_4`
      (`self.Colums` false)
      (`self.Colums` true)
      (`self.Colums` false true)
      (`self.Colums` true true))))

(fn `WallSetup`
  (params (Horizontal :type Boolean) (Upper :type Boolean))
  (locals (HorizontalLocal :type Boolean) (UpperLocal :type Boolean))
  (bind (_offset_x _offset_y) (`KismetMathLibrary.BreakVector2D` (`self.GridOffset`)))
  (bind _wallsize (`self.WallSize`))
  (bind (_tilesize_x _tilesize_y) (`KismetMathLibrary.BreakVector2D` (`self.TileSize`)))
  (bind _upperlocal (`local.UpperLocal`))
  (bind (_roomsize_x _roomsize_y) (`KismetMathLibrary.BreakVector2D` (`self.RoomSize`)))
  (bind (_roomsize_x_2 _roomsize_y_2) (`KismetMathLibrary.BreakVector2D` (`self.RoomSize`)))
  (bind _upperlocal_2 (`local.UpperLocal`))
  (bind _horizontallocal (`local.HorizontalLocal`))
  (bind _returnvalue (/ _tilesize_x 2.0))
  (bind _returnvalue_2 (/ _tilesize_y 2.0))
  (set `local.HorizontalLocal` Horizontal)
  (set `local.UpperLocal` Upper)
  (for _index (range (`KismetMathLibrary.FTrunc` (`KismetMathLibrary.SelectFloat` _roomsize_x_2 _roomsize_y_2 (`local.HorizontalLocal`))))
    (bind _returnvalue_3 (* (`KismetMathLibrary.Conv_IntToDouble` _index) _wallsize))
    (bind _returnvalue_4 (`AddComponent|NODE_AddStaticMeshComponent-7` :`RelativeTransform` (`KismetMathLibrary.MakeTransform` (`KismetMathLibrary.MakeVector` (- (`KismetMathLibrary.SelectFloat` (+ _returnvalue_3 _returnvalue_2) (- (`KismetMathLibrary.SelectFloat` (* _wallsize _roomsize_x) 0.0 _upperlocal_2) _returnvalue) _horizontallocal) _offset_x) (- (`KismetMathLibrary.SelectFloat` (- (`KismetMathLibrary.SelectFloat` (* _wallsize _roomsize_y) 0.0 _upperlocal_2) _returnvalue_2) (+ _returnvalue_3 _returnvalue) _horizontallocal) _offset_y)) (`KismetMathLibrary.MakeRotator` 0.0 0.0 (`KismetMathLibrary.SelectFloat` (`KismetMathLibrary.SelectFloat` -90.0 90.0 _upperlocal) (`KismetMathLibrary.SelectFloat` 180.0 0.0 _upperlocal) (`local.HorizontalLocal`))))))
    (`StaticMeshComponent.SetStaticMesh` _returnvalue_4 "/Game/ModularEnv/Walls/Wall_1.Wall_1")
    (`PrimitiveComponent.SetMaterial` _returnvalue_4 0 "/Game/ModularEnv/RoomPreview_M.RoomPreview_M")))