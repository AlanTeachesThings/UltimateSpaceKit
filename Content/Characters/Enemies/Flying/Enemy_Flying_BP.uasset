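; Flying enemy Blueprint that runs the Enemy_Small_BT behavior tree on its AI controller and handles taking damage and dying.
; Any damage lowers Health and halts AI movement by clearing the TargetLocation blackboard key and stopping the controller.
; A surviving hit raises HitReact briefly, while a lethal one sets IsDying.
; A separate Die event destroys the actor and is not called within this graph.
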(event `self.ReceiveBeginPlay`
  (bind _output_get (set `self.AI_Cont` (`AIBlueprintHelperLibrary.GetAIController` self)))
  (`AIController.RunBehaviorTree` _output_get "/Game/Characters/Enemies/Small/AI/Enemy_Small_BT.Enemy_Small_BT")
  (add `self.OnTakeAnyDamage` (delegate `OnTakeDamage`)))

(event `OnTakeDamage` :!signature `self.OnTakeAnyDamage`
  (params (DamagedActor :type "Actor Object Reference") (Damage :type "Float (single-precision)") (DamageType :type "DamageType Object Reference") (InstigatedBy :type "Controller Object Reference") (DamageCauser :type "Actor Object Reference"))
  (bind _output_get (set `self.Health` (- (`self.Health`) Damage)))
  (if (<= _output_get 0.0)
    (set `self.isDying` true)
    (`self.StopAIMovement`)
    (else
      (`self.StopAIMovement`)
      (set `self.HitReact` true)
      (`KismetSystemLibrary.Delay` 0.3)
      (set `self.HitReact` false))))

(event `Die`
  (`self.K2_DestroyActor`))

(fn `StopAIMovement`
  (bind _ai_cont (`self.AI_Cont`))
  (`BlackboardComponent.ClearValue` (`AIBlueprintHelperLibrary.GetBlackboard` _ai_cont) "TargetLocation")
  (`Controller.StopMovement` _ai_cont))

(fn `UserConstructionScript`)